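; Base pickup item actor that adds itself to the inventory component of an overlapping actor implementing BPI_Inventory.
; Sphere overlap on authority starts a server-to-client event chain that calls the component's add function and sets the picked-up flag, whose OnRep destroys the actor.
; Pickup sound plays locally in 2D, or routes through the component's server or multicast events when replication is enabled.
; A helper function refreshes the inventory widget after successful pickup, but nothing here calls it.
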(event OnComponentBeginOverlap(Sphere)
  (params (OverlappedComponent :type Primitive%20Component%20Object%20Reference) (OtherActor :type Actor%20Object%20Reference) (OtherComp :type Primitive%20Component%20Object%20Reference) (OtherBodyIndex :type Integer) (bFromSweep :type Boolean) (SweepResult :type Hit%20Result%20Structure%20%28by%20ref%29))
  (if (Utilities|DoesObjectImplementInterface OtherActor "/Game/PirateGame/Program/Blueprints/Core/Inventory/BPI_Inventory.BPI_Inventory_C")
    (Utilities|FlowControl|Sequence
      (:then_0
        (Networking|SwitchHasAuthority
          (:Authority
            (CallFunction|ServerAddItemonInventory (Actor|GetComponentbyClass OtherActor "/Game/PirateGame/Program/Blueprints/Core/Inventory/C_Inventory_Component.C_Inventory_Component_C") self))))
      (:then_1
        (if (not (Variables|Default|GetReplicate%20Pick%20Up%20Sound?))
          (Audio|PlaySound2D "/Engine/VREditor/Sounds/UI/Camera_Shutter.Camera_Shutter" 1.0 1.0 0.0 0 0))))))

(event Custom|Server_AddItemOnInventory
  (params (Target :type C%20Inventory%20Component%20Object%20Reference) (NewItem :type BP%20Master%20Item%20Object%20Reference%20%28by%20ref%29))
  ;[1 1 1] Server Handling to Add the Items to Player Inventory
  (CallFunction|ClientAddItemtoInventory Target NewItem))

(event Custom|Client%20Add%20Item%20to%20Inventory
  (params (Target :type C%20Inventory%20Component%20Object%20Reference) (NewItem :type BP%20Master%20Item%20Object%20Reference%20%28by%20ref%29))
  ;[1 1 1] Server Handling to Add the Items to Player Inventory
  (Default|FAddItemtoInventory Target NewItem)
  (CallFunction|FCheckifSoundShouldMulticast Target)
  (Variables|Default|SetItem%20Picked%20Up%20Successfully? true))

(event Custom|Client%20Update%20Inventory
  (params (Inventory%20Component%20In :type C%20Inventory%20Component%20Object%20Reference))
  ;[1 1 1] Server Handling to Add the Items to Player Inventory
)

(event EventBeginPlay)

(event Collision|EventActorBeginOverlap
  (params (OtherActor :type Actor%20Object%20Reference)))

(event EventTick
  (params (DeltaSeconds :type Float%20%28single-precision%29)))

(fn ConstructionScript)

(fn FCheckifSoundShouldMulticast
  (params (InputPin :type C%20Inventory%20Component%20Object%20Reference))
  (bind _itemmeshshow (Variables|Default|GetItemMeshShow))
  (bind _returnvalue (Transformation|GetWorldLocation _itemmeshshow))
  (if (Variables|Default|GetReplicate%20Pick%20Up%20Sound?)
    (Networking|SwitchHasAuthority
      (:Authority
        (Default|MCPickUpSound InputPin "/Engine/VREditor/Sounds/UI/Camera_Shutter.Camera_Shutter" _returnvalue))
      (:Remote
        (Default|ServerPickUpSound InputPin "/Engine/VREditor/Sounds/UI/Click_on_Button.Click_on_Button" _returnvalue)))))

(fn FUpdateInventoryifOpen
  (params (Inventory%20Component%20In :type C%20Inventory%20Component%20Object%20Reference))
  (bind _wd_inventory (Variables|/Game/PirateGame/Program/Blueprints/Core/Inventory/C_Inventory_Component.C_Inventory_Component_C|GetWD_Inventory Inventory%20Component%20In))
  (Utilities|IsValid _wd_inventory
    (:Is%20Valid
      (if (Variables|Default|GetItem%20Picked%20Up%20Successfully?)
        (Default|FUpdate _wd_inventory (Variables|/Game/PirateGame/Program/Blueprints/Core/Inventory/C_Inventory_Component.C_Inventory_Component_C|GetInventory Inventory%20Component%20In))
        (Development|PrintString "Update")
        (else
          (Development|PrintString "Item not Picked Up Successfully"))))
    (:Is%20Not%20Valid
      (Development|PrintString "not Valid"))))

(fn OnRepItemPickedUpSuccessfully?
  (Actor|DestroyActor))