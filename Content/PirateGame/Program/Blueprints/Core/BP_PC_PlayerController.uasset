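; Player controller for the pirate game that creates the master UI and provides a key-triggered self-damage input.
; On BeginPlay, CreateClientWidget builds WD_Master for player controller 0, stores it as MasterWidget and adds it to the viewport.
; Pressing P calls the ServerDamage event, which applies a fixed amount of damage to the controlled pawn.
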(event Custom|ServerDamage
  (params (BaseDamage :type Float%20%28single-precision%29))
  (Game|Damage|ApplyDamage (Pawn|GetControlledPawn) BaseDamage 0 0))

(event Custom|Create%20Client%20Widget
  (bind _returnvalue (UserInterface|CreateWidget "/Game/PirateGame/Program/UI/WD_Master.WD_Master_C" (Game|GetPlayerController 0)))
  (bind _output_get (Variables|Default|SetMasterWidget _returnvalue))
  (Utilities|IsValid _output_get
    (:Is%20Valid
      (UserInterface|Viewport|AddtoViewport _output_get 0))))

(event EventBeginPlay
  (CallFunction|CreateClientWidget))

(event Input|KeyboardEvents|P
  (params (Key :type Key%20Structure :default "None"))
  (:Pressed
    (CallFunction|ServerDamage 1e+01)))

(fn ConstructionScript)