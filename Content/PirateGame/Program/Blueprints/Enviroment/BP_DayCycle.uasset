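; BP_DayCycle is an actor that drives the day-night cycle by rotating the sun light over time.
; On BeginPlay it starts a looping timer at a configurable refresh interval that calls Update Sun Position.
; Each tick of that timer adds local pitch to the referenced sunlight, scaled by speed and multiplier, then tells the referenced sky sphere to update its sun direction.
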(event Custom|Day%20Night%20Cycle
  (Utilities|Time|SetTimerbyFunctionName 0 "Update Sun Position" (Variables|Default|GetRefresh%20Time%20In%20Seconds) true))

(event EventBeginPlay
  (CallFunction|DayNightCycle))

(fn ConstructionScript)

(fn UpdateSunPosition
  (Transformation|AddActorLocalRotation (Variables|Default|GetRef%20Sunlight) (Math|Rotator|MakeRotator 0.0 (* (Variables|Default|GetSunlight%20Speed%20Multiplier) (Variables|Default|GetSunlight%20Speed)) 0.0) false false)
  (Default|UpdateSunDirection (Variables|Default|GetRef%20Skysphere)))